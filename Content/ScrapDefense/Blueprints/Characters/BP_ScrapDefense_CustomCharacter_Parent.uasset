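; Parent character Blueprint for Scrap Defense characters, holding shared combat and movement stats.
; SetCharacterBaseStats stores health, ranged and melee attack parameters and move speed, starts current health at maximum and applies the speed to CharacterMovement's MaxWalkSpeed.
; MeleeAttack and RangedAttack are empty functions, and the event graph and construction script have no logic.
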(event EventBeginPlay)

(event Collision|EventActorBeginOverlap
  (params (OtherActor :type Actor%20Object%20Reference)))

(event EventTick
  (params (DeltaSeconds :type Float%20%28single-precision%29)))

(fn ConstructionScript)

(fn MeleeAttack)

(fn RangedAttack)

(fn SetCharacterBaseStats
  (params (MaxHealthPoints :type Float%20%28double-precision%29) (CanRangedAttack? :type Boolean) (RangedAttackMinDistance :type Float%20%28double-precision%29) (RangedAttackMaxDistance :type Float%20%28double-precision%29) (RangedAttackHitPoints :type Float%20%28double-precision%29) (RangedAttackRate :type Float%20%28double-precision%29) (CanMeleeAttack? :type Boolean) (MeleeAttackMinDistance :type Float%20%28double-precision%29) (MeleeAttackMaxDistance :type Float%20%28double-precision%29) (MeleeAttackHitPoints :type Float%20%28double-precision%29) (MeleeAttackRate :type Float%20%28double-precision%29) (MoveSpeed :type Float%20%28double-precision%29))
  (bind _output_get (Variables|[CUSTOMCHARACTER]|SetMaxHealthPoints MaxHealthPoints))
  (Variables|[CUSTOMCHARACTER]|SetCurrentHealthPoints _output_get)
  (Variables|[CUSTOMCHARACTER]|SetCanRangedAttack? CanRangedAttack?)
  (Variables|[CUSTOMCHARACTER]|SetRangedAttackMinDistance RangedAttackMinDistance)
  (Variables|[CUSTOMCHARACTER]|SetRangedAttackMaxDistance RangedAttackMaxDistance)
  (Variables|[CUSTOMCHARACTER]|SetRangedAttackHitPoints RangedAttackHitPoints)
  (Variables|[CUSTOMCHARACTER]|SetRangedAttackRate RangedAttackRate)
  (Variables|[CUSTOMCHARACTER]|SetCanMeleeAttack? CanMeleeAttack?)
  (Variables|[CUSTOMCHARACTER]|SetMeleeAttackMinDistance MeleeAttackMinDistance)
  (Variables|[CUSTOMCHARACTER]|SetMeleeAttackMaxDistance MeleeAttackMaxDistance)
  (Variables|[CUSTOMCHARACTER]|SetMeleeAttackHitPoints MeleeAttackHitPoints)
  (Variables|[CUSTOMCHARACTER]|SetMeleeAttackRate MeleeAttackRate)
  (bind _output_get_2 (Variables|[CUSTOMCHARACTER]|SetMoveSpeed MoveSpeed))
  (Variables|/Script/Engine.CharacterMovementComponent|SetMaxWalkSpeed (Variables|Character|GetCharacterMovement) _output_get_2))