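; Base enemy character for Scrap Defense that pursues the player, with health and move speed driven by variables.
; On BeginPlay it fills current health to maximum, applies its move speed to CharacterMovement and starts a stored looping timer.
; That timer repeatedly reissues AIMoveTo with the player character as target actor to keep the chase going.
; The health bar update function is an empty stub, and no damage or death logic is present.
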(event Custom|ChasePlayer
  ;[0 0.6288 1 1 40] BEGIN PLAY
  ;;[0.1059 0.1059 0.1059] Permet de poursuivre le joueur. Actualise la position toute les 0.25 sec
  ;;;[1 1 1] Destination ou Target Actor, pas les deux simultanement
  (AI|AIMoveTo self "0, 0, 0" (Game|GetPlayerCharacter 0) 5.0 false))

(event EventBeginPlay
  ;[0 0.6288 1 1 40] BEGIN PLAY
  ;;[0.1059 0.1059 0.1059] Permet de poursuivre le joueur. Actualise la position toute les 0.25 sec
  (bind _returnvalue (Utilities|Time|SetTimerbyEvent (delegate Custom|ChasePlayer) 0.25 true))
  (Variables|Déplacements|SetChase%20Timer _returnvalue)
  ;;[0.1059 0.1059 0.1059] Spawn avec la vie maximum
  (Variables|Default|SetCurrentHealthPoints (Variables|Default|GetMaxHealthPoints))
  ;;[0.1059 0.1059 0.1059] Définit la vitesse de déplacement de l'ennemi (les ennemis + fort vont + lentement)
  (Variables|/Script/Engine.CharacterMovementComponent|SetMaxWalkSpeed (Variables|Character|GetCharacterMovement) (Variables|Default|GetMoveSpeed)))

(fn ConstructionScript)

(fn UpdateHealthBar)