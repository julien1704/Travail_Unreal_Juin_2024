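; Player character for Scrap Defense that moves relative to camera yaw and turns to face the mouse cursor.
; BeginPlay sets up Enhanced Input, camera pitch limit and stats, fills a toggleable stats HUD, and caches controller and game instance.
; Tick traces under the cursor to set actor yaw and CharacterRotation for the animation blendspace.
; Attacks, shield and pause only print; pause widget logic is unwired, damage tint and TakeItem are unfinished.
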(event Custom|SetActorRotationToCursor
  (bind _returnvalue (Game|GetPlayerController 0))
  (bind _returnvalue_2 (Transformation|GetActorLocation))
  (bind _hitresult (Game|Player|GetHitResultUnderCursorbyChannel _returnvalue "TraceTypeQuery1" true))
  (bind _impactpoint (Collision|BreakHitResult _hitresult))
  (bind _returnvalue_3 (Math|Rotator|FindLookatRotation _returnvalue_2 _impactpoint))
  ;[1 0.7804 0.1765 1 35] Permet que le personnage fasse toujours face au curseur de la souris [APPELÉ DANS L'EVENT TICK]
  (Transformation|SetActorRotation (Math|Rotator|MakeRotator 0.0 0.0 (.yaw _returnvalue_3)))
  ;;[0.1059 0.1059 0.1059] Variable utilisée dans l'Animation Blueprint pour détecter où regarde le personnage et servir de direction au Blendspace
  (Variables|[CUSTOMCHARACTER]|SetCharacterRotation (Math|Rotator|MakeRotator 0.0 0.0 (.yaw _returnvalue_3))))

(event Input|EnhancedActionEvents|EnhancedInputActionIA_ScrapDefense_Shield
  (params (ActionValue :type Boolean) (ElapsedSeconds :type Float%20%28double-precision%29) (TriggeredSeconds :type Float%20%28double-precision%29) (InputAction :type Input%20Action%20Object%20Reference :default "/Game/ScrapDefense/Blueprints/Inputs/IA_ScrapDefense_Shield.IA_ScrapDefense_Shield"))
  ;[0.9804 0.1137 0.1137 1 35] F KEYBOARD KEY - SHIELD
  (:Started
    (Development|PrintString "F KEYBOARD KEY - SHIELD")))

(event Input|EnhancedActionEvents|EnhancedInputActionIA_ScrapDefense_Display_Stats_Of_Player
  (params (ActionValue :type Boolean) (ElapsedSeconds :type Float%20%28double-precision%29) (TriggeredSeconds :type Float%20%28double-precision%29) (InputAction :type Input%20Action%20Object%20Reference :default "/Game/ScrapDefense/Blueprints/Inputs/IA_ScrapDefense_Display_Stats_Of_Player.IA_ScrapDefense_Display_Stats_Of_Player"))
  ;[0.9804 0.1137 0.1137 1 35] X KEYBOARD KEY - DISPLAY PLAYER'S STATS
  (:Started
    (switch Utilities|FlowControl|Switch|SwitchonESlateVisibility (Widget|GetVisibility (Variables|[CUSTOMCHARACTER]|GetPlayerStatsWidget))
      (:Hidden
        (Widget|SetVisibility (Variables|[CUSTOMCHARACTER]|GetPlayerStatsWidget) "SelfHitTestInvisible")
        (Development|PrintString "PLAYER'S STATS HUD - VISIBLE NOT HIT (SELF ONLY)"))
      (:SelfHitTestInvisible
        (Widget|SetVisibility (Variables|[CUSTOMCHARACTER]|GetPlayerStatsWidget) "Hidden")
        (Development|PrintString "PLAYER'S STATS HUD - HIDDEN")))))

(event Input|EnhancedActionEvents|EnhancedInputActionIA_ScrapDefense_RangedAttack
  (params (ActionValue :type Boolean) (ElapsedSeconds :type Float%20%28double-precision%29) (TriggeredSeconds :type Float%20%28double-precision%29) (InputAction :type Input%20Action%20Object%20Reference :default "/Game/ScrapDefense/Blueprints/Inputs/IA_ScrapDefense_RangedAttack.IA_ScrapDefense_RangedAttack"))
  ;[0.9804 0.1137 0.1137 1 35] LEFT MOUSE BUTTON CLICK - RANGED ATTACK
  (:Started
    (Development|PrintString "LEFT MOUSE BUTTON - RANGED ATTACK")))

(event Input|EnhancedActionEvents|EnhancedInputActionIA_ScrapDefense_MeleeAttack
  (params (ActionValue :type Boolean) (ElapsedSeconds :type Float%20%28double-precision%29) (TriggeredSeconds :type Float%20%28double-precision%29) (InputAction :type Input%20Action%20Object%20Reference :default "/Game/ScrapDefense/Blueprints/Inputs/IA_ScrapDefense_MeleeAttack.IA_ScrapDefense_MeleeAttack"))
  ;[0.9804 0.1137 0.1137 1 35] RIGHT MOUSE BUTTON CLICK - MELEE ATTACK
  (:Started
    (Development|PrintString "RIGHT MOUSE BUTTON - MELEE ATTACK")))

(event Input|EnhancedActionEvents|EnhancedInputActionIA_ScrapDefense_Move
  (params (ActionValue :type Vector%202D%20Structure) (ElapsedSeconds :type Float%20%28double-precision%29) (TriggeredSeconds :type Float%20%28double-precision%29) (InputAction :type Input%20Action%20Object%20Reference :default "/Game/ScrapDefense/Blueprints/Inputs/IA_ScrapDefense_Move.IA_ScrapDefense_Move"))
  (bind _returnvalue (Pawn|GetControlRotation :!class /Script/Engine.Pawn))
  (bind _yaw (Math|Rotator|BreakRotator _returnvalue))
  (bind _returnvalue_2 (Math|Rotator|MakeRotator 0.0 0.0 _yaw))
  ;[0.9804 0.1137 0.1137 1 35] ZSQD KEYBOARD KEYS - PLAYER'S MOVEMENTS
  (:Triggered
    (Pawn|Input|AddMovementInput (Math|Vector|GetRightVector _returnvalue_2) (.x ActionValue) false)
    (Pawn|Input|AddMovementInput (Math|Vector|GetForwardVector _returnvalue_2) (.y ActionValue) false)))

(event Input|EnhancedActionEvents|EnhancedInputActionIA_ScrapDefense_Pause
  (params (ActionValue :type Boolean) (ElapsedSeconds :type Float%20%28double-precision%29) (TriggeredSeconds :type Float%20%28double-precision%29) (InputAction :type Input%20Action%20Object%20Reference :default "/Game/ScrapDefense/Blueprints/Inputs/IA_ScrapDefense_Pause.IA_ScrapDefense_Pause"))
  ;[0.9804 0.1137 0.1137 1 35] ESCAPE AND P KEYBOARD KEYS - PAUSE MENU
  (:Started
    (Development|PrintString "ESCAPE OR P KEYBOARD KEYS - PAUSE MENU")))

(event EventTick
  (params (DeltaSeconds :type Float%20%28single-precision%29))
  ;[1 0.7804 0.1765 1 40] TICK -> CALL ON EVERY FRAME /!\ EN DERNIER RECOURS, A EVITER SI POSSIBLE /!\
  (CallFunction|SetActorRotationtoCursor))

(event EventBeginPlay
  ;[0 0.6288 1 1 40] BEGIN PLAY
  ;;[0.1059 0.1059 0.1059] ADD THE MAPPING CONTEXT TO SET THE INPUTS
  (Input|AddMappingContext (PlayerController|LocalPlayerSubsystems|GetEnhancedInputLocalPlayerSubsystem (Game|GetPlayerController 0)) "/Game/ScrapDefense/Blueprints/Inputs/IMC_ScrapDefense_Player.IMC_ScrapDefense_Player" 0 "(bIgnoreAllPressedKeysUntilRelease=True,bForceImmediately=False)")
  ;;[0.1059 0.1059 0.1059] SET THE CAMERA ANGLE
  (Variables|/Script/Engine.PlayerCameraManager|SetViewPitchMax (Game|GetPlayerCameraManager 0) -35.0)
  ;;[0.1059 0.1059 0.1059] SET PLAYER'S STATS
  (Variables|Default|SetCurrentHealthPoints (Variables|Default|GetMaxHealthPoints))
  (Variables|/Script/Engine.CharacterMovementComponent|SetMaxWalkSpeed (Variables|Character|GetCharacterMovement) (Variables|Default|GetMoveSpeed))
  ;;[0.1059 0.1059 0.1059] CREATE THE HUD WIDGET AND SET IT
  (bind _returnvalue (UserInterface|CreateWidget "/Game/ScrapDefense/WBP_ScrapDefense_Player_Stats_HUD.WBP_ScrapDefense_Player_Stats_HUD_C"))
  (bind _output_get (Variables|[CUSTOMCHARACTER]|SetPlayerStatsWidget _returnvalue))
  ;;[0.1059 0.1059 0.1059] SET CUSTOM CHARACTER BASE STATS TO THE HUD WIDGET (TO DO : MAKE A FUNCTION)
  (Variables|/Game/ScrapDefense/WBP_ScrapDefense_Player_Stats_HUD.WBP_ScrapDefense_Player_Stats_HUD_C|SetCustomCharacter _output_get self)
  (Variables|/Game/ScrapDefense/WBP_ScrapDefense_Player_Stats_HUD.WBP_ScrapDefense_Player_Stats_HUD_C|SetMaxHealthPoints _output_get (Variables|Default|GetMaxHealthPoints))
  (Variables|/Game/ScrapDefense/WBP_ScrapDefense_Player_Stats_HUD.WBP_ScrapDefense_Player_Stats_HUD_C|SetCurrentHealthPoints _output_get (Variables|Default|GetCurrentHealthPoints))
  (Variables|/Game/ScrapDefense/WBP_ScrapDefense_Player_Stats_HUD.WBP_ScrapDefense_Player_Stats_HUD_C|SetCanRangedAttack? _output_get (Variables|Default|GetCanRangedAttack?))
  (Variables|/Game/ScrapDefense/WBP_ScrapDefense_Player_Stats_HUD.WBP_ScrapDefense_Player_Stats_HUD_C|SetRangedAttackMinDistance _output_get (Variables|Default|GetRangedAttackMinDistance))
  (Variables|/Game/ScrapDefense/WBP_ScrapDefense_Player_Stats_HUD.WBP_ScrapDefense_Player_Stats_HUD_C|SetRangedAttackMaxDistance _output_get (Variables|Default|GetRangedAttackMaxDistance))
  (Variables|/Game/ScrapDefense/WBP_ScrapDefense_Player_Stats_HUD.WBP_ScrapDefense_Player_Stats_HUD_C|SetRangedAttackHitPoints _output_get (Variables|Default|GetRangedAttackHitPoints))
  (Variables|/Game/ScrapDefense/WBP_ScrapDefense_Player_Stats_HUD.WBP_ScrapDefense_Player_Stats_HUD_C|SetRangedAttackRate _output_get (Variables|Default|GetRangedAttackRate))
  (Variables|/Game/ScrapDefense/WBP_ScrapDefense_Player_Stats_HUD.WBP_ScrapDefense_Player_Stats_HUD_C|SetCanMeleeAttack? _output_get (Variables|Default|GetCanMeleeAttack?))
  (Variables|/Game/ScrapDefense/WBP_ScrapDefense_Player_Stats_HUD.WBP_ScrapDefense_Player_Stats_HUD_C|SetMeleeAttackMinDistance _output_get (Variables|Default|GetMeleeAttackMinDistance))
  (Variables|/Game/ScrapDefense/WBP_ScrapDefense_Player_Stats_HUD.WBP_ScrapDefense_Player_Stats_HUD_C|SetMeleeAttackMaxDistance _output_get (Variables|Default|GetMeleeAttackMaxDistance))
  (Variables|/Game/ScrapDefense/WBP_ScrapDefense_Player_Stats_HUD.WBP_ScrapDefense_Player_Stats_HUD_C|SetMeleeAttackHitPoints _output_get (Variables|Default|GetMeleeAttackHitPoints))
  (Variables|/Game/ScrapDefense/WBP_ScrapDefense_Player_Stats_HUD.WBP_ScrapDefense_Player_Stats_HUD_C|SetMeleeAttackRate _output_get (Variables|Default|GetMeleeAttackRate))
  (Variables|/Game/ScrapDefense/WBP_ScrapDefense_Player_Stats_HUD.WBP_ScrapDefense_Player_Stats_HUD_C|SetMoveSpeed _output_get (Variables|Default|GetMoveSpeed))
  ;;[0.1059 0.1059 0.1059] ADD WIDGET TO VIEWPORT
  (UserInterface|Viewport|AddtoViewport _output_get 0)
  ;;[0.1059 0.1059 0.1059] GET PLAYER'S CONTROLLER AND SAVE IT AS VARIABLE
  (bind _aspc_scrap_defense_my_controller (Utilities|Casting|CastToPC_ScrapDefense_MyController (Game|GetPlayerController 0)))
  (bind _output_get_2 (Variables|[CUSTOMCHARACTER]|SetControllerRef _aspc_scrap_defense_my_controller))
  ;;[0.1059 0.1059 0.1059] GET MOUSE'S WIDGET AND SAVE IT AS VARIABLE
  (Variables|[CUSTOMCHARACTER]|SetCursorWidget (Variables|/Game/ScrapDefense/Blueprints/PC_ScrapDefense_MyController.PC_ScrapDefense_MyController_C|GetCursorWidget _output_get_2))
  (Input|SetInputModeGameandUI _output_get_2 0 "DoNotLock" true false)
  ;;[0.1059 0.1059 0.1059] GET THE GAME INSTANCE AND SAVE IT AS VARIABLE (TO SAVE DATA)
  (bind _asgi_scrap_defense_game_instance (Utilities|Casting|CastToGI_ScrapDefense_GameInstance (Game|GetGameInstance)))
  (Variables|[CUSTOMCHARACTER]|SetGameInstanceRef _asgi_scrap_defense_game_instance))

(fn ConstructionScript)

(fn AlterScreenColorwithPV
  (Variables|/Script/Engine.PostProcessComponent|SetSettings (Variables|Default|GetDamagePostProcess) (Utilities|Struct|MakePostProcessSettings (Math|Color|Lerp(LinearColor) "(R=1.000000,G=0.427083,B=0.427083,A=1.000000)" "(R=1.000000,G=1.000000,B=1.000000,A=1.000000)" (/ 0.0 0.0)))))

(fn TakeItem)