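; Relic item for Scrap Defense that expires on its own or turns into a portal.
; BeginPlay waits for LifeTime, then destroys the actor.
; GeneratePortal spawns an actor of class PortalType and destroys the relic immediately.
; ChangePlayerStat is an empty function, and the construction script only calls its parent.
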(event EventBeginPlay
  (Utilities|FlowControl|Delay (Variables|Default|GetLifeTime))
  (Actor|DestroyActor))

(fn ConstructionScript
  (|CallParentFunction))

(fn ChangePlayerStat)

(fn GeneratePortal
  (Game|SpawnActorfromClass (Variables|Default|GetPortalType) (Math|Transform|MakeTransform "0, 0, 0" "0, 0, 0" "1.000000,1.000000,1.000000") "Undefined" "MultiplyWithRoot" 0 0)
  (Actor|DestroyActor))